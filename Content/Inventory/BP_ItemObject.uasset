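; BP_ItemObject represents an inventory item, exposing its data through getter functions.
; The getters read two structs: SItemDetails for general data such as dimensions, type, weight, count and sounds, and SOutfitCharacteristics for outfit stats including max weight.
; GetIcon picks the normal or rotated icon from the Rotated flag, returning nothing unless both icons are valid.
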(fn GetDimensions
  (return (.Dimensions (Utilities|Struct|BreakS_ItemDetails (Variables|Default|GetS_ItemDetails)))))

(fn GetIcon
  (bind _s_itemdetails (Variables|Default|GetS_ItemDetails))
  (bind (_icon _iconratated _rotated_) (Utilities|Struct|BreakS_ItemDetails _s_itemdetails))
  (Utilities|IsValid _icon
    (:Is%20Valid
      (Utilities|IsValid _iconratated
        (:Is%20Valid
          (return (select _rotated_ _iconratated _icon)))
        (:Is%20Not%20Valid
          (return 0))))
    (:Is%20Not%20Valid
      (return 0))))

(fn GetItemClass
  (return (.ItemClass (Utilities|Struct|BreakS_ItemDetails (Variables|Default|GetS_ItemDetails)))))

(fn GetItemType
  (return (.ItemType (Utilities|Struct|BreakS_ItemDetails (Variables|Default|GetS_ItemDetails)))))

(fn GetEquipmentSound
  (return (.EquipmentSound (Utilities|Struct|BreakS_ItemDetails (Variables|Default|GetS_ItemDetails)))))

(fn GetDropSound
  (return (.DropSound (Utilities|Struct|BreakS_ItemDetails (Variables|Default|GetS_ItemDetails)))))

(fn GetRotationIcon
  (return (.IconRatated (Utilities|Struct|BreakS_ItemDetails (Variables|Default|GetS_ItemDetails)))))

(fn GetOutfitCharacteristics
  (return (Variables|Default|GetS_OutfitCharacteristics)))

(fn GetCondition
  (return (.Condition (Utilities|Struct|BreakS_ItemDetails (Variables|Default|GetS_ItemDetails)))))

(fn GetWeight
  (return (.Weight (Utilities|Struct|BreakS_ItemDetails (Variables|Default|GetS_ItemDetails)))))

(fn GetName
  (return (.Name (Utilities|Struct|BreakS_ItemDetails (Variables|Default|GetS_ItemDetails)))))

(fn GetMaxWeight
  (return (.MaxWeight (Utilities|Struct|BreakOutfitCharacteristics (Variables|Default|GetS_OutfitCharacteristics)))))

(fn GetItemDetails
  (return (Variables|Default|GetS_ItemDetails)))

(fn GetSoundOfUse
  (return (Utilities|Struct|BreakS_ItemDetails (Variables|Default|GetS_ItemDetails))))

(fn GetCount
  (return (Utilities|Struct|BreakS_ItemDetails (Variables|Default|GetS_ItemDetails))))