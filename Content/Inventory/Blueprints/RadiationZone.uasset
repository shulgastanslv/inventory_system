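; Radiation hazard zone that drains the first-person character's health and shows a post-process effect while they are inside its box.
; While occupied, a delayed Tick loop plays a sound at world origin and sums outfit and helmet radiation protection from the inventory.
; With zero protection, damage delay depends on the zone's high, average or low level.
; Otherwise, damage applies only when protection fails to exceed that level's threshold.
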(event OnComponentBeginOverlap(Box)
  (params (OverlappedComponent :type Primitive%20Component%20Object%20Reference) (OtherActor :type Actor%20Object%20Reference) (OtherComp :type Primitive%20Component%20Object%20Reference) (OtherBodyIndex :type Integer) (bFromSweep :type Boolean) (SweepResult :type Hit%20Result%20Structure%20%28by%20ref%29))
  (bind _asfirst_person_character (Utilities|Casting|CastToFirstPersonCharacter OtherActor))
  (Variables|Private|SetRadiationZone true)
  (Variables|Private|SetFirst%20Person%20Character _asfirst_person_character)
  (Rendering|SetVisibility (Variables|Default|GetPostProcess) true false))

(event OnComponentEndOverlap(Box)
  (params (OverlappedComponent :type Primitive%20Component%20Object%20Reference) (OtherActor :type Actor%20Object%20Reference) (OtherComp :type Primitive%20Component%20Object%20Reference) (OtherBodyIndex :type Integer))
  (Utilities|Casting|CastToFirstPersonCharacter OtherActor)
  (Variables|Private|SetRadiationZone false)
  (Rendering|SetVisibility (Variables|Default|GetPostProcess) false false))

(event Custom|Average%20Radiation%20Level%20Damage
  (if (not (.Average%20Level (CallFunction|RadiationLevelwithOutfit (Variables|Public|GetRadiation%20Level))))
    (Utilities|FlowControl|Delay 0.05)
    (CallFunction|RadiationDamage (Variables|Private|GetRadiation%20Damage%20))))

(event Custom|Radiation%20Damage%20without%20Outfit
  (bind _radiation_level (Variables|Public|GetRadiation%20Level))
  (bind _radiation_damage_ (Variables|Private|GetRadiation%20Damage%20))
  (bind (_high_level _average_level _low_level) (CallFunction|RadiationLevelWithoutOutfit _radiation_level))
  (if _high_level
    (Utilities|FlowControl|Delay 0.2)
    (CallFunction|RadiationDamage _radiation_damage_)
    (elif _average_level
      (Utilities|FlowControl|Delay 0.3)
      (CallFunction|RadiationDamage _radiation_damage_)
      (elif _low_level
        (Utilities|FlowControl|Delay 0.5)
        (CallFunction|RadiationDamage _radiation_damage_)))))

(event Custom|High%20Radiation%20Level%20Damage
  (if (not (.High%20Level (CallFunction|RadiationLevelwithOutfit (Variables|Public|GetRadiation%20Level))))
    (Utilities|FlowControl|Delay 0.09)
    (CallFunction|RadiationDamage (Variables|Private|GetRadiation%20Damage%20))))

(event Custom|Low%20Radiation%20Level%20Damage
  (if (not (.Low%20Level (CallFunction|RadiationLevelwithOutfit (Variables|Public|GetRadiation%20Level))))
    (Utilities|FlowControl|Delay 0.01)
    (CallFunction|RadiationDamage (Variables|Private|GetRadiation%20Damage%20))))

(event EventTick
  (params (DeltaSeconds :type Float%20%28single-precision%29))
  (bind _radiation_level (Variables|Public|GetRadiation%20Level))
  (bind (_highlevel _averagelevel _lowlevel) (Utilities|Struct|BreakS_RadiationLevels _radiation_level))
  (if (Variables|Private|GetRadiationZone)
    (Utilities|FlowControl|Delay 0.2)
    (Audio|PlaySoundatLocation "/Game/Inventory/Sounds/Cue/RadiatonZone.RadiatonZone" "0, 0, 0" "0, 0, 0" 1.0 1.0 0.0 0 0 0)
    (bind _output_get (Variables|Private|SetOutfit%20Radiation%20Characteristics (+ (.Radiation (Utilities|Struct|BreakOutfitCharacteristics (Default|GetOutfitCharacteristics (Variables|/Game/FirstPersonBP/Blueprints/FirstPersonCharacter.FirstPersonCharacter_C|GetInventoryComponent (stale OnComponentBeginOverlap(Box) _asfirst_person_character))))) (.Radiation (Utilities|Struct|BreakOutfitCharacteristics (Default|GetHelmetCharacteristics (Variables|/Game/FirstPersonBP/Blueprints/FirstPersonCharacter.FirstPersonCharacter_C|GetInventoryComponent (stale OnComponentBeginOverlap(Box) _asfirst_person_character))))))))
    (if (== _output_get 0.0)
      (CallFunction|RadiationDamageWithoutOutfit)
      (elif _highlevel
        (CallFunction|HighRadiationLevelDamage)
        (elif _averagelevel
          (CallFunction|AverageRadiationLevelDamage)
          (elif _lowlevel
            (CallFunction|LowRadiationLevelDamage)))))))

(fn ConstructionScript)

(fn RadiationLevelWithoutOutfit
  (params (S_RadiationLevels :type S%20Radiation%20Levels%20Structure%20%28by%20ref%29))
  (bind (_highlevel _averagelevel _lowlevel) (Utilities|Struct|BreakS_RadiationLevels S_RadiationLevels))
  (bind _outfit_radiation_characteristics (Variables|Private|GetOutfit%20Radiation%20Characteristics))
  (bind _returnvalue (== _outfit_radiation_characteristics 0.0))
  (return (and _returnvalue _highlevel) (and _returnvalue _averagelevel) (and _returnvalue _lowlevel)))

(fn RadiationDamage
  (params (Damage :type Float%20%28single-precision%29))
  (bind _first_person_character (Variables|Private|GetFirst%20Person%20Character))
  (bind _healthcomponent (Variables|/Game/FirstPersonBP/Blueprints/FirstPersonCharacter.FirstPersonCharacter_C|GetHealthComponent _first_person_character))
  (Variables|/Game/Inventory/Components/HealthComponent.HealthComponent_C|SetHealth _healthcomponent (- (Variables|/Game/Inventory/Components/HealthComponent.HealthComponent_C|GetHealth _healthcomponent) Damage)))

(fn RadiationLevelwithOutfit
  (params (S_RadiationLevels :type S%20Radiation%20Levels%20Structure%20%28by%20ref%29))
  (bind (_highlevel _averagelevel _lowlevel) (Utilities|Struct|BreakS_RadiationLevels S_RadiationLevels))
  (bind _outfit_radiation_characteristics (Variables|Private|GetOutfit%20Radiation%20Characteristics))
  (return (and (> _outfit_radiation_characteristics 0.5) _highlevel) (and (> _outfit_radiation_characteristics 0.3) _averagelevel) (and (> _outfit_radiation_characteristics 0.1) _lowlevel)))